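; MeshWidgetNoPlugin is an actor Blueprint that displays a widget's rendered output on a static mesh through a material.
; On BeginPlay it applies the material to the mesh's first slot and creates a dynamic instance of it.
; Every Tick it feeds the Widget's render target into that instance's texture parameter.
; An unconnected timer node is noted as an alternative to Tick.
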(event `self.ReceiveBeginPlay`
  (bind _dynamicmaterial (`self.DynamicMaterial`))
  (bind _staticmesh (`self.StaticMesh`))
  ;[0.1354 0.1206 0] Begin Play
  ;[1 1 1] Setting Material To Render
  (`PrimitiveComponent.SetMaterial` _staticmesh 0 _dynamicmaterial)
  ;[0.1875 0.1875 0.1875] Create Dynamic Material For Static Mesh
  (bind _returnvalue (`PrimitiveComponent.CreateDynamicMaterialInstance` _staticmesh 0 _dynamicmaterial "None"))
  (set `self.MaterialInstance` _returnvalue))

(event `self.ReceiveTick`
  (params (DeltaSeconds :type "Float (single-precision)"))
  ;[0.1354 0.1206 0] Even Tick
  ;[0.1875 0.1875 0.1875] Set Texture and Render Material On Mesh
  (`MaterialInstanceDynamic.SetTextureParameterValue` (`self.MaterialInstance`) (`self.TextureParmName`) (`WidgetComponent.GetRenderTarget` (`self.Widget`))))

(fn `UserConstructionScript`)